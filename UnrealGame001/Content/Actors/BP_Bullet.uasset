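; BP_Bullet is a bullet actor that damages whatever it overlaps, then destroys itself.
; On BeginPlay it binds the Collision component's begin-overlap event and starts a one-shot timer from its Time variable.
; The overlap handler applies BaseDamage, crediting the instigator's controller and passing the instigator, rather than the bullet, as damage causer.
; The construction script sizes Collision from the Scale variable.
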(event `self.ReceiveBeginPlay`
  (add `PrimitiveComponent.OnComponentBeginOverlap` (`self.Collision`) (`|CreateDelegate` :!event `HandleOverlap`))
  (`KismetSystemLibrary.K2_SetTimerDelegate` (`|CreateDelegate` :!event `K2_DestroyActor`) (`self.Time`)))

(event `HandleOverlap`
  (params (OverlappedComponent :type "PrimitiveComponent Object Reference") (OtherActor :type "Actor Object Reference") (OtherComp :type "PrimitiveComponent Object Reference") (OtherBodyIndex :type Integer) (bFromSweep :type Boolean) (SweepResult :type "HitResult Structure (by ref)"))
  (`GameplayStatics.ApplyDamage` OtherActor (`self.BaseDamage`) (`self.GetInstigatorController`) (`self.GetInstigator`))
  (`self.K2_DestroyActor`))

(fn `UserConstructionScript`
  (`SceneComponent.SetWorldScale3D` (`self.Collision`) (`self.Scale`)))