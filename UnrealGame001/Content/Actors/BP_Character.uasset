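; Base-style character Blueprint that carries a rifle and handles attacking, hurt and death.
; BeginPlay spawns the weapon class through a child actor component, caches it and the anim Blueprint, destroying itself if either cast fails, then binds health, bullet and animation events.
; CharacterAttack forwards to the weapon.
; CharacterDeath notifies animation and weapon and disables collision; CanPickupHealth always returns false.
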(event `self.ReceiveBeginPlay`
  (bind _weaponchildactorcomponent (`self.WeaponChildActorComponent`))
  (bind _bp_healthcomponent (`self.BP_HealthComponent`))
  (`ChildActorComponent.SetChildActorClass` _weaponchildactorcomponent (`self.WeaponClass`))
  (bind _asbp_rifle (cast `/Game/Actors/BP_Rifle` (`ChildActorComponent.ChildActor` _weaponchildactorcomponent))
    (:`then`
      (set `self.CurrentWeapon` _asbp_rifle)
      (bind _asabp_character (cast `/Game/Art/ABP_Character` (`SkeletalMeshComponent.GetAnimInstance` (`self.Mesh`)))
        (:`then`
          (set `self.AnimBP` _asabp_character)
          (add `/Game/Components/BP_HealthComponent.OnHurt` _bp_healthcomponent (delegate `Testing`))
          (add `/Game/Components/BP_HealthComponent.OnDeath` _bp_healthcomponent (`|CreateDelegate` :!event `Testing`))
          ;[1 1 1] new
          (add `/Game/Actors/BP_Rifle.OnBulletCreated` (`self.CurrentWeapon`) (`|CreateDelegate` (`self.AnimBP`) :!event `Fire Animation`))
          (add `/Game/Components/BP_HealthComponent.OnHurt` (`self.BP_HealthComponent`) (`|CreateDelegate` (`self.AnimBP`) :!event `HitAnimation`))
          (add `/Game/Art/ABP_Character.OnAnimEnded` (`self.AnimBP`) (`|CreateDelegate` (`self.CurrentWeapon`) :!event `FinishAttack`))
          (add `/Game/Components/BP_HealthComponent.OnDeath` (`self.BP_HealthComponent`) (`|CreateDelegate` :!event `CharacterDeath`)))
        (:`CastFailed`
          (`KismetSystemLibrary.PrintString` "need correct animmation")
          (`self.K2_DestroyActor`))))
    (:`CastFailed`
      (`KismetSystemLibrary.PrintString` "no weapon")
      (`self.K2_DestroyActor`))))

(event `Testing`
  (params (Amount :type "Float (double-precision)"))
  (`KismetSystemLibrary.PrintString` (`KismetStringLibrary.Conv_DoubleToString` Amount)))

(event `CharacterDeath`
  (params (junk :type "Float (double-precision)"))
  (`/Game/Art/ABP_Character.DeathAnimation` (`self.AnimBP`) junk)
  (`/Game/Actors/BP_Rifle.SetDeath` (`self.CurrentWeapon`) junk)
  (`self.SetActorEnableCollision` false))

(fn `CanPickupHealth`
  (params (OtherActor :type "Actor Object Reference"))
  (returns (Yes :type Boolean))
  (return false))

(fn `CharacterAttack`
  (`/Game/Actors/BP_Rifle.Attack` (`self.CurrentWeapon`)))

(fn `UserConstructionScript`)