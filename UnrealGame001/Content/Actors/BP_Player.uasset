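; BP_Player is the player-controlled character, handling camera look, yaw-relative movement and an attack input that calls CharacterAttack.
; On BeginPlay it creates and shows a HUD widget for its player controller, then binds delegates to the health component's hurt and death events.
; Without a player controller, it prints an error and destroys itself.
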(event `self.ReceiveBeginPlay`
  (bind _bp_healthcomponent (`self.BP_HealthComponent`))
  (`parent.ReceiveBeginPlay`)
  (bind _asplayer_controller (cast `PlayerController` (`self.GetController`))
    (:`then`
      (bind _returnvalue (`|CreateWidget` (`self.WidgetClass`) _asplayer_controller))
      (bind _output_get (set `self.HUDWidget` _returnvalue))
      (`UserWidget.AddToViewport` _output_get 0)
      (add `/Game/Components/BP_HealthComponent.OnHurt` _bp_healthcomponent (`|CreateDelegate` (`self.HUDWidget`) :!event `SetHealth`))
      (add `/Game/Components/BP_HealthComponent.OnDeath` _bp_healthcomponent (`|CreateDelegate` (`self.HUDWidget`) :!event `SetHealth`)))
    (:`CastFailed`
      (`KismetSystemLibrary.PrintString` "need a plyer controller")
      (`self.K2_DestroyActor`))))

(event `InputAxis|Turn`
  (params (AxisValue :type "Float (single-precision)"))
  (`self.AddControllerYawInput` AxisValue))

(event `InputAxis|LookUp`
  (params (AxisValue :type "Float (single-precision)"))
  (`self.AddControllerPitchInput` AxisValue))

(event `InputAxis|Forward`
  (params (AxisValue :type "Float (single-precision)"))
  (bind (_returnvalue_roll _returnvalue_pitch _returnvalue_yaw) (`KismetMathLibrary.BreakRotator` (`self.GetControlRotation`)))
  (`self.AddMovementInput` (`KismetMathLibrary.GetForwardVector` (`KismetMathLibrary.MakeRotator` 0.0 0.0 _returnvalue_yaw)) AxisValue))

(event `InputAxis|Right`
  (params (AxisValue :type "Float (single-precision)"))
  (bind (_returnvalue_roll _returnvalue_pitch _returnvalue_yaw) (`KismetMathLibrary.BreakRotator` (`self.GetControlRotation`)))
  (`self.AddMovementInput` (`KismetMathLibrary.GetRightVector` (`KismetMathLibrary.MakeRotator` 0.0 0.0 _returnvalue_yaw)) AxisValue))

(event `InputAction|Attack`
  (params (Key :type "Key Structure"))
  (:`Pressed`
    (`self.CharacterAttack`)))

(fn `UserConstructionScript`
  (`parent.UserConstructionScript`))