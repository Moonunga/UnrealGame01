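; BP_Pickup is a generic pickup actor that reacts when something overlaps its box collision and then removes itself.
; BeginPlay binds the overlap event, and the overlap handler checks CanPickup before calling HandlePickup and PostPickup.
; It works as an overridable template: CanPickup accepts any actor by default, HandlePickup is an empty hook, and PostPickup destroys the actor.
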(event `self.ReceiveBeginPlay`
  (add `PrimitiveComponent.OnComponentBeginOverlap` (`self.BoxCollision`) (`|CreateDelegate` :!event `HandleOverlap`)))

(event `HandlePickup`
  (params (OtherActor :type "Actor Object Reference") (SweepResult :type "HitResult Structure")))

(event `PostPickup`
  (`self.K2_DestroyActor`))

(event `HandleOverlap`
  (params (OverlappedComponent :type "PrimitiveComponent Object Reference") (OtherActor :type "Actor Object Reference") (OtherComp :type "PrimitiveComponent Object Reference") (OtherBodyIndex :type Integer) (bFromSweep :type Boolean) (SweepResult :type "HitResult Structure (by ref)"))
  (if (`self.CanPickup` OtherActor)
    (`self.HandlePickup` OtherActor SweepResult)
    (`self.PostPickup`)))

(fn `CanPickup`
  (params (OtherActor :type "Actor Object Reference"))
  (returns (Yes :type Boolean))
  (return true))

(fn `UserConstructionScript`)